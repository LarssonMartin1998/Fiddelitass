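; BP_ButtonToStart is a physical push button for motion controllers that starts the game by loading TheStage_P.
; A BP_MotionController overlapping Cylinder2 plays a timeline that lowers the cylinder, with a moving flag blocking retriggers.
; On finishing, a DoOnce-gated sequence reverses the press, fades the camera out and opens the level after a delay.
; A separate ClearDoOnceThing event can reset the gate.
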(event OnComponentBeginOverlap(Cylinder2)
  (params (OverlappedComponent :type Primitive%20Component%20Object%20Reference) (OtherActor :type Actor%20Object%20Reference) (OtherComp :type Primitive%20Component%20Object%20Reference) (OtherBodyIndex :type Integer) (bFromSweep :type Boolean) (SweepResult :type Hit%20Result%20Structure%20%28by%20ref%29))
  (if (not (Variables|Default|GetButtonIsMoving))
    (Utilities|Casting|CastToBP_MotionController OtherActor)
    (bind _alpha (Timeline|ButtonAnimation PlayFromStart)
      (:Update
        (Variables|Default|SetButtonIsMoving true)
        (Transformation|SetRelativeLocation (Variables|Default|GetCylinder2) (Math|Vector|MakeVector 0.0 0.0 (Math|Float|Lerp 58.0 53.0 _alpha)) false false))
      (:Finished
        (Variables|Default|SetButtonIsMoving false)
        (Utilities|FlowControl|DoOnce false
          (:Completed
            (Utilities|FlowControl|Delay 0.2)
            (CallFunction|ReverseButtonAnimation)
            (CameraFades|StartCameraFade :self (Game|GetPlayerCameraManager 0) :ToAlpha 1.0 :Duration 1.0 :bHoldWhenFinished true)
            (Utilities|FlowControl|Delay 2.0)
            (Game|OpenLevel(byName) "TheStage_P")))))))

(event Custom|ReverseButtonAnimation
  (bind _alpha (Timeline|ButtonAnimation ReverseFromEnd)
    (:Update
      (Variables|Default|SetButtonIsMoving true)
      (Transformation|SetRelativeLocation (Variables|Default|GetCylinder2) (Math|Vector|MakeVector 0.0 0.0 (Math|Float|Lerp 58.0 53.0 _alpha)) false false))
    (:Finished
      (Variables|Default|SetButtonIsMoving false)
      (Utilities|FlowControl|DoOnce false
        (:Completed
          (Utilities|FlowControl|Delay 0.2)
          (CallFunction|ReverseButtonAnimation)
          (CameraFades|StartCameraFade :self (Game|GetPlayerCameraManager 0) :ToAlpha 1.0 :Duration 1.0 :bHoldWhenFinished true)
          (Utilities|FlowControl|Delay 2.0)
          (Game|OpenLevel(byName) "TheStage_P"))))))

(event Custom|ClearDoOnceThing
  (Utilities|FlowControl|DoOnce false) ; enters at Reset
)

(event Collision|EventActorBeginOverlap
  (params (OtherActor :type Actor%20Object%20Reference)))

(event EventTick
  (params (DeltaSeconds :type Float%20%28single-precision%29)))

(fn ConstructionScript)